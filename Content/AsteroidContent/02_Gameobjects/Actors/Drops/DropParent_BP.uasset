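; DropParent_BP is the base class for pickup drops that the player's spaceship collects by touch.
; At BeginPlay it rolls a random on-screen lifetime, counts it down in Tick and destroys itself when time runs out.
; Box overlap with a Spaceship_BP calls Effect on that ship, then destroys the drop.
; Effect is empty here, leaving the actual bonus to child Blueprints.
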(event OnComponentBeginOverlap(Box)
  (params (OverlappedComponent :type Primitive%20Component%20Object%20Reference) (OtherActor :type Actor%20Object%20Reference) (OtherComp :type Primitive%20Component%20Object%20Reference) (OtherBodyIndex :type Integer) (bFromSweep :type Boolean) (SweepResult :type Hit%20Result%20Structure%20%28by%20ref%29))
  (bind _asspaceship_bp (Utilities|Casting|CastToSpaceship_BP OtherActor))
  (CallFunction|Effect _asspaceship_bp)
  (Actor|DestroyActor))

(event EventBeginPlay
  (Variables|Default|SettimeOnScreen (Math|Random|RandomFloatinRange (Variables|Default|GetminTimeOnScreen) (Variables|Default|GetmaxTimeOnScreen))))

(event Collision|EventActorBeginOverlap
  (params (OtherActor :type Actor%20Object%20Reference)))

(event EventTick
  (params (DeltaSeconds :type Float%20%28single-precision%29))
  (bind _output_get (Variables|Default|SettimeOnScreen (- (Variables|Default|GettimeOnScreen) DeltaSeconds)))
  (if (<= _output_get 0.0)
    (Actor|DestroyActor)))

(fn ConstructionScript)

(fn Effect
  (params (Player :type Spaceship%20BP%20Object%20Reference)))