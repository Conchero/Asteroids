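; FirerateUpgrade_BP is a drop that upgrades the fire rate of the player it is applied to.
; Its Effect function gets the player's shoot component and sets its fire rate to the current value minus FireRateUpgrade.
; The event graph holds only disabled default nodes, and the construction script just calls its parent.
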(event EventBeginPlay
  (|CallParentFunction) ; This node is disabled and will not be called.\nDrag off pins to build functionality.
)

(event Collision|EventActorBeginOverlap
  (params (OtherActor :type Actor%20Object%20Reference))
  (|CallParentFunction OtherActor) ; This node is disabled and will not be called.\nDrag off pins to build functionality.
)

(event EventTick
  (params (DeltaSeconds :type Float%20%28single-precision%29))
  (|CallParentFunction DeltaSeconds) ; This node is disabled and will not be called.\nDrag off pins to build functionality.
)

(fn ConstructionScript
  (|CallParentFunction))

(fn Effect
  (params (Player :type Spaceship%20BP%20Object%20Reference))
  (bind _returnvalue (Class|Spaceship|GetShootComponent Player))
  (Class|ShootComponent|SetFireRate _returnvalue (- (Class|ShootComponent|GetCurrentFireRate _returnvalue) (Variables|Default|GetfireRateUpgrade))))