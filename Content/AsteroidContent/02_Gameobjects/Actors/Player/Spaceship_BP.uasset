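; Player spaceship Blueprint for an asteroid game that owns the player's UI and handles restarting after death or victory.
; On BeginPlay it creates Player_UI, links it to itself and adds it to the viewport.
; SetUIHealth and SetUIGameOver events forward updates to that widget when it is valid.
; Any key press calls Revive if the ship is dead or AsteroidGameMode_BP reports a win.
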(event EventBeginPlay
  (bind _returnvalue (UserInterface|CreateWidget "/Game/AsteroidContent/04_Widget/Player_UI.Player_UI_C" (Game|GetPlayerController 0)))
  (bind _output_get (Variables|Default|SetPlayerUI _returnvalue))
  (Variables|/Game/AsteroidContent/04_Widget/Player_UI.Player_UI_C|SetlinkedPlayer _output_get self)
  (UserInterface|Viewport|AddtoViewport _output_get 0))

(event Collision|EventActorBeginOverlap
  (params (OtherActor :type Actor%20Object%20Reference)))

(event EventTick
  (params (DeltaSeconds :type Float%20%28single-precision%29)))

(event EventSetUIHealth
  (bind _playerui (Variables|Default|GetPlayerUI))
  (Utilities|IsValid _playerui
    (:Is%20Valid
      (Default|SetHealth _playerui))))

(event EventSetUIGameOver
  (params (show :type Boolean))
  (bind _playerui (Variables|Default|GetPlayerUI))
  (Utilities|IsValid _playerui
    (:Is%20Valid
      (Default|SetGameOver _playerui show))))

(event Input|KeyboardEvents|AnyKey
  (params (Key :type Key%20Structure :default "None"))
  (:Pressed
    (bind _asasteroid_game_mode_bp (Utilities|Casting|CastToAsteroidGameMode_BP (Game|GetGameMode)))
    (if (or (Class|Spaceship|GetIsDead) (Class|AsteroidGameMode|GetGameWin _asasteroid_game_mode_bp))
      (Class|Spaceship|Revive))))

(fn ConstructionScript)